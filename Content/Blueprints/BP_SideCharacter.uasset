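; BP_SideCharacter is a side character that starts a conversation when another actor walks into its interaction trigger box.
; On overlap, it looks up the RFDialogueComponent on the other actor and, if one exists, starts a dialogue between that component and its own DialogueComponent.
; The dialogue always uses the DGraph_Test_Bartender graph, and the returned context is stored in DialogueContext.
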(event OnComponentBeginOverlap(InteractionTriggerBox)
  (params (OverlappedComponent :type Primitive%20Component%20Object%20Reference) (OtherActor :type Actor%20Object%20Reference) (OtherComp :type Primitive%20Component%20Object%20Reference) (OtherBodyIndex :type Integer) (bFromSweep :type Boolean) (SweepResult :type Hit%20Result%20Structure%20%28by%20ref%29))
  (if (!= OtherActor self)
    (CallFunction|StartDialogue OtherActor)))

(fn ConstructionScript)

(fn StartDialogue
  (params (OtherActor :type Actor%20Object%20Reference))
  (bind _output_get (Variables|Dialogue|SetOtherParticipant (Actor|GetComponentbyClass OtherActor "/Script/RoyalFlush.RFDialogueComponent")))
  (Utilities|IsValid _output_get
    (:Is%20Valid
      (Utilities|FlowControl|Sequence
        (:then_0
          (bind _returnvalue (Class|DlgManager|StartDialogue2 "/Game/Blueprints/Test/DGraph_Test_Bartender.DGraph_Test_Bartender" (Variables|Dialogue|GetOtherParticipant) (Variables|Dialogue|GetDialogueComponent)))
          (Variables|Dialogue|SetDialogueContext _returnvalue))))))