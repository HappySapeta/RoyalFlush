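; BP_PlayerCharacter is the player character Blueprint, handling the start and end of dialogue interactions with another participant.
; When an interaction starts, it stores the other participant, creates and shows a WBP_Dialogue widget, binds to its quit event and disables movement.
; On quit, it removes the widget, notifies the participant that the interaction finished and restores walking movement.
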(event Custom|OnQuitInteraction
  ;[0.15 0.15 0.15 0.5] On Interaction Started
  (Widget|RemovefromParent (stale EventOnInteractionStarted _output_get))
  (Class|RFCharacter|OnInteractionFinished (Variables|Default|GetDialogueParticipant))
  (Pawn|Components|CharacterMovement|SetMovementMode (Variables|Character|GetCharacterMovement) "MOVE_Walking" 0))

(event EventOnInteractionStarted
  (params (Other :type RF%20Character%20Object%20Reference))
  ;[0.15 0.15 0.15 0.5] On Interaction Started
  (Variables|Default|SetDialogueParticipant Other)
  (bind _returnvalue (UserInterface|CreateWidget "/Game/UI/WBP_Dialogue.WBP_Dialogue_C"))
  (bind _output_get (Variables|Default|SetDialogueInteractionWidget _returnvalue))
  (Utilities|FlowControl|Sequence
    (:then_0
      (UserInterface|Viewport|AddtoViewport _output_get 0))
    (:then_1
      (EventDispatchers|BindEventtoOnQuitInteraction _output_get (delegate Custom|OnQuitInteraction)))
    (:then_2
      (Pawn|Components|CharacterMovement|DisableMovement (Variables|Character|GetCharacterMovement)))))

(fn ConstructionScript)